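; Projected menu actor that turns on by scaling up its mesh, then pulses its bands, and opens a prompt when clicked.
; Clicking any of its three meshes spawns a BP_Prompt linked back to it, plays a sound and swaps materials, gated by a DoOnce.
; ResetPrompt restores the default materials and re-arms that gate, while Repair applies a repair look.
; Hovering the center brightens it only while no prompt is open.
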(event OnClicked(StaticMesh)
  (params (TouchedComponent :type Primitive%20Component%20Object%20Reference) (ButtonPressed :type Key%20Structure :default "None"))
  ;[1 1 1] Call Spawn on click
  (CallFunction|SpawnPrompt))

(event OnClicked(Bands)
  (params (TouchedComponent :type Primitive%20Component%20Object%20Reference) (ButtonPressed :type Key%20Structure :default "None"))
  ;[1 1 1] Call Spawn on click
  (CallFunction|SpawnPrompt))

(event OnClicked(Center)
  (params (TouchedComponent :type Primitive%20Component%20Object%20Reference) (ButtonPressed :type Key%20Structure :default "None"))
  ;[1 1 1] Call Spawn on click
  (CallFunction|SpawnPrompt))

(event OnBeginCursorOver(Center)
  (params (TouchedComponent :type Primitive%20Component%20Object%20Reference))
  (if (not (Variables|Default|GetbIsPromptOpen))
    (Rendering|Material|SetMaterial (Variables|Default|GetCenter) 0 "/Game/Materials/ProjectedMenuRotating_Bright.ProjectedMenuRotating_Bright")))

(event OnEndCursorOver(Center)
  (params (TouchedComponent :type Primitive%20Component%20Object%20Reference))
  (if (not (Variables|Default|GetbIsPromptOpen))
    (Rendering|Material|SetMaterial (Variables|Default|GetCenter) 0 "/Game/Materials/ProjectedMenuRotating.ProjectedMenuRotating")))

(event Custom|TurnOn
  ;[1 1 1] Scale up to appear like it turns on. Initiate bands movement after/
  (bind _alpha (Timeline|ProjectorDriver PlayFromStart)
    (:Update
      (Transformation|SetWorldScale3D (Variables|Default|GetStaticMesh) (Math|Vector|Lerp(Vector) "0, 0, 0" "0.250000,0.250000,0.250000" _alpha)))
    (:Finished
      (CallFunction|Modulate))))

(event Custom|Modulate
  ;[1 1 1] Move bands
  (bind _alpha (Timeline|BandsDriver Play)
    (:Update
      (Transformation|SetRelativeScale3D (Variables|Default|GetBands) (Math|Vector|Lerp(Vector) "1.000000,1.000000,1.000000" "1.050000,1.050000,1.050000" _alpha)))))

(event Custom|SpawnPrompt
  ;[1 1 1] Spawn prompt
  (Utilities|FlowControl|DoOnce false
    (:Completed
      (bind _returnvalue (Game|SpawnActorfromClass "/Game/Blueprints/BP_Prompt.BP_Prompt_C" (Transformation|GetActorTransform) "Undefined" 0 0))
      (Variables|/Game/Blueprints/BP_Prompt.BP_Prompt_C|SetParentMenu _returnvalue self)
      (Rendering|Material|SetMaterial (Variables|Default|GetStaticMesh) 0 "/Game/Materials/ProjectedMenu_Inst.ProjectedMenu_Inst")
      (Rendering|Material|SetMaterial (Variables|Default|GetCenter) 0 "/Game/Materials/ProjectedMenuRotating_Inst.ProjectedMenuRotating_Inst")
      (Audio|PlaySoundatLocation "/Game/Sounds/CUE_OpenSound.CUE_OpenSound" (Transformation|GetActorLocation) "0, 0, 0" 1.0 1.0 0.0 0 0 0)
      (Variables|Default|SetbIsPromptOpen true))))

(event Custom|ResetPrompt
  ;[1 1 1] Spawn prompt
  (Variables|Default|SetbIsPromptOpen false)
  (Rendering|Material|SetMaterial (Variables|Default|GetStaticMesh) 0 "/Game/Materials/ProjectedMenu.ProjectedMenu")
  (Rendering|Material|SetMaterial (Variables|Default|GetCenter) 0 "/Game/Materials/ProjectedMenuRotating.ProjectedMenuRotating")
  (Utilities|FlowControl|DoOnce false) ; enters at Reset
)

(event Custom|Repair
  (Rendering|Material|SetMaterial (Variables|Default|GetBands) 0 "/Game/Materials/ProjectedMenu_Repairs.ProjectedMenu_Repairs")
  (Rendering|Material|SetMaterial (Variables|Default|GetCenter) 0 "/Game/Materials/ProjectedMenuRotating.ProjectedMenuRotating"))

(fn ConstructionScript)