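; BP_Prompt is a Yes/No confirmation prompt actor that asks its parent menu to carry out or cancel a repair.
; Clicking Yes calls Repair on ParentMenu, while NO calls ResetPrompt, with beep and close sounds played at the actor's location.
; Either click destroys the prompt.
; Cursor-over events swap each button component between normal and glow materials.
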(event OnClicked(NO)
  (params (TouchedComponent :type Primitive%20Component%20Object%20Reference) (ButtonPressed :type Key%20Structure :default "None"))
  (bind _parentmenu (Variables|Default|GetParentMenu))
  ;[1 1 1] Click events
  (Utilities|IsValid _parentmenu
    (:Is%20Valid
      (Default|ResetPrompt _parentmenu)
      (Audio|PlaySoundatLocation "/Game/Sounds/CUE_CloseSound.CUE_CloseSound" (Transformation|GetActorLocation) "0, 0, 0" 1.0 1.0 0.0 0 0 0))
    (:Is%20Not%20Valid
      _))
  (Actor|DestroyActor))

(event OnClicked(Yes)
  (params (TouchedComponent :type Primitive%20Component%20Object%20Reference) (ButtonPressed :type Key%20Structure :default "None"))
  (bind _parentmenu (Variables|Default|GetParentMenu))
  ;[1 1 1] Click events
  (Utilities|IsValid _parentmenu
    (:Is%20Valid
      (Default|Repair _parentmenu))
    (:Is%20Not%20Valid
      _))
  (Audio|PlaySoundatLocation "/Game/Sounds/CUE_PositiveBeep.CUE_PositiveBeep" (Transformation|GetActorLocation) "0, 0, 0" 1.0 1.0 0.0 0 0 0)
  (Audio|PlaySoundatLocation "/Game/Sounds/CUE_CloseSound.CUE_CloseSound" (Transformation|GetActorLocation) "0, 0, 0" 1.0 1.0 0.0 0 0 0)
  (Actor|DestroyActor))

(event OnBeginCursorOver(Yes)
  (params (TouchedComponent :type Primitive%20Component%20Object%20Reference))
  ;[1 1 1] Mouseover events
  ;;[1 1 1] Yes material on mouseover
  (Rendering|Material|SetMaterial (Variables|Default|GetYes) 0 "/Game/Materials/Prompt_Glow.Prompt_Glow"))

(event OnEndCursorOver(Yes)
  (params (TouchedComponent :type Primitive%20Component%20Object%20Reference))
  ;[1 1 1] Mouseover events
  ;;[1 1 1] Yes material on mouseover
  (Rendering|Material|SetMaterial (Variables|Default|GetYes) 0 "/Game/Materials/Prompt.Prompt"))

(event OnBeginCursorOver(NO)
  (params (TouchedComponent :type Primitive%20Component%20Object%20Reference))
  ;[1 1 1] Mouseover events
  ;;[1 1 1] No material on mouseover
  (Rendering|Material|SetMaterial (Variables|Default|GetNO) 0 "/Game/Materials/Prompt_Glow.Prompt_Glow"))

(event OnEndCursorOver(NO)
  (params (TouchedComponent :type Primitive%20Component%20Object%20Reference))
  ;[1 1 1] Mouseover events
  ;;[1 1 1] No material on mouseover
  (Rendering|Material|SetMaterial (Variables|Default|GetNO) 0 "/Game/Materials/Prompt.Prompt"))

(fn ConstructionScript)