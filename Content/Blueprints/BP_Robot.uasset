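; BP_Robot is a clickable spider robot that spawns and turns on a BP_ProjectedMenu when first clicked.
; A Sphere swaps the body material on hover; clicking restores it, shrinks the sphere and plays an eye-open animation with servo sounds.
; Two chained timelines loop a material-driven eye movement with random pauses.
; While the menu is open, Tick periodically replays an eyelid idle animation and servo sound.
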(event OnBeginCursorOver(Sphere)
  (params (TouchedComponent :type Primitive%20Component%20Object%20Reference))
  ;[1 1 1 1 24] Mouseover changes color to indicate clickable object
  (if (not (Variables|Default|GetbIsMenuOpen))
    (Rendering|Material|SetMaterial (Variables|Default|GetSkeletalMesh) 0 "/Game/Materials/SP-07_Body_Inst.SP-07_Body_Inst")))

(event OnEndCursorOver(Sphere)
  (params (TouchedComponent :type Primitive%20Component%20Object%20Reference))
  ;[1 1 1 1 24] Mouseover changes color to indicate clickable object
  (if (not (Variables|Default|GetbIsMenuOpen))
    (Rendering|Material|SetMaterial (Variables|Default|GetSkeletalMesh) 0 "/Game/Materials/SP-07_Body.SP-07_Body")))

(event OnClicked(Sphere)
  (params (TouchedComponent :type Primitive%20Component%20Object%20Reference) (ButtonPressed :type Key%20Structure :default "None"))
  (bind _returnvalue (Transformation|GetActorLocation))
  (bind _skeletalmesh (Variables|Default|GetSkeletalMesh))
  ;[1 1 1] On click, spawn projected menu, open eyes, reset material, hide sphere to prevent interference with clicking
  (Utilities|FlowControl|DoOnce false
    (:Completed
      (Variables|Default|SetbIsMenuOpen true)
      (bind _returnvalue_2 (Game|SpawnActorfromClass "/Game/Blueprints/BP_ProjectedMenu.BP_ProjectedMenu_C" (Transformation|GetActorTransform) "AlwaysSpawn" 0 0))
      (Variables|Default|SetProjectedMenu _returnvalue_2)
      (Default|Turnon _returnvalue_2)
      (Components|Animation|PlayAnimation _skeletalmesh "/Game/Meshes/SpiderBot/SpiderbotForMenu_Anim_SP-07Skeleton_SP07EyeOpen.SpiderbotForMenu_Anim_SP-07Skeleton_SP07EyeOpen" false)
      (Rendering|Material|SetMaterial _skeletalmesh 0 "/Game/Materials/SP-07_Body.SP-07_Body")
      (Components|Sphere|SetSphereRadius (Variables|Default|GetSphere) 5.0 true)
      (Audio|PlaySoundatLocation "/Game/Sounds/CUE_ServoSingle.CUE_ServoSingle" _returnvalue "0, 0, 0" 1.0 1.0 0.0 0 0 0)
      (Utilities|FlowControl|Delay 0.2)
      (Audio|PlaySoundatLocation "/Game/Sounds/CUE_OpenSound.CUE_OpenSound" _returnvalue "0, 0, 0" 1.0 1.0 0.0 0 0 0))))

(event EventBeginPlay
  (bind _alpha (Timeline|EyeDriver Play)
    (:Update
      (Rendering|Material|SetScalarParameterValueonMaterials (Variables|Default|GetSkeletalMesh) "EyeMovement" (Math|Float|Lerp 0.0 0.1 _alpha)))
    (:Finished
      (Utilities|FlowControl|Delay (Math|Random|RandomFloatinRange 1.5 3.0))
      (bind _alpha_2 (Timeline|EyeReverseDriver PlayFromStart)
        (:Update
          (Rendering|Material|SetScalarParameterValueonMaterials (Variables|Default|GetSkeletalMesh) "EyeMovement" (Math|Float|Lerp 0.1 0.0 _alpha_2)))
        (:Finished
          (Utilities|FlowControl|Delay (Math|Random|RandomFloatinRange 3.0 5.0))
          (Timeline|EyeDriver PlayFromStart))))))

(event EventTick
  (params (DeltaSeconds :type Float%20%28single-precision%29))
  (bind _eyelidtimelimit (Variables|Default|GetEyeLidTimeLimit))
  ;[1 1 1] Play eyelid movements
  (if (Variables|Default|GetbIsMenuOpen)
    (Variables|Default|SetElapsedTime (+ DeltaSeconds (Variables|Default|GetElapsedTime)))
    (if (>= (+ DeltaSeconds (Variables|Default|GetElapsedTime)) _eyelidtimelimit)
      (Variables|Default|SetElapsedTime (- (Variables|Default|GetElapsedTime) _eyelidtimelimit))
      (Components|Animation|PlayAnimation (Variables|Default|GetSkeletalMesh) "/Game/Meshes/SpiderBot/SpiderbotForMenu_Anim_SP-07Skeleton_SP07EyeIdle.SpiderbotForMenu_Anim_SP-07Skeleton_SP07EyeIdle" false)
      (Audio|PlaySoundatLocation "/Game/Sounds/CUE_ServoDouble.CUE_ServoDouble" (Transformation|GetActorLocation) "0, 0, 0" 1.0 1.0 0.0 0 0 0))))

(fn ConstructionScript)